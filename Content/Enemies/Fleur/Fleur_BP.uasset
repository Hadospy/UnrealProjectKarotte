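; Fleur is a side-scroller flipbook enemy that patrols horizontally, reverses on capsule hits and shoots at the player.
; Tick updates animation, movement, player distance and a directional Impulse vector; the Capsule overlap sets SeePlayer, driving a DoOnce-gated shot that re-arms after a delay.
; ColliderAR overlap turns it around and clears detection.
; Box overlap kills it and bounces the player upward; DeadCAC provides a separate suicide-animation death.
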(event OnComponentHit(CapsuleComponent)
  (params (HitComponent :type Primitive%20Component%20Object%20Reference) (OtherActor :type Actor%20Object%20Reference) (OtherComp :type Primitive%20Component%20Object%20Reference) (NormalImpulse :type Vector :default "0, 0, 0") (Hit :type Hit%20Result%20Structure%20%28by%20ref%29))
  (Variables|Default|SetIsMovingRight (not (Variables|Default|GetIsMovingRight))))

(event OnComponentBeginOverlap(Box)
  (params (OverlappedComponent :type Primitive%20Component%20Object%20Reference) (OtherActor :type Actor%20Object%20Reference) (OtherComp :type Primitive%20Component%20Object%20Reference) (OtherBodyIndex :type Integer) (bFromSweep :type Boolean) (SweepResult :type Hit%20Result%20Structure%20%28by%20ref%29))
  (Utilities|Casting|CastTo2DSideScrollerCharacter OtherActor)
  (Utilities|FlowControl|DoOnce false
    (:Completed
      (Variables|Default|SetIsDead true)
      (Character|LaunchCharacter (Game|GetPlayerCharacter 0) "0, 0,800.000000" false true)
      (Variables|Default|SetAnimState "NewEnumerator1")
      (CallFunction|AnimationUpdate)
      (Pawn|Components|CharacterMovement|DisableMovement (Variables|Character|GetCharacterMovement))
      (Utilities|FlowControl|Delay 0.6)
      (Actor|DestroyActor))))

(event OnComponentEndOverlap(Capsule)
  (params (OverlappedComponent :type Primitive%20Component%20Object%20Reference) (OtherActor :type Actor%20Object%20Reference) (OtherComp :type Primitive%20Component%20Object%20Reference) (OtherBodyIndex :type Integer))
  (Utilities|Casting|CastTo2DSideScrollerCharacter OtherActor)
  (Variables|Default|SetSeePlayer false)
  (Pawn|Components|CharacterMovement|SetMovementMode (Variables|Character|GetCharacterMovement) "MOVE_Walking" 0)
  (Variables|Default|SetAnimState "NewEnumerator2")
  (CallFunction|AnimationUpdate))

(event OnComponentBeginOverlap(Capsule)
  (params (OverlappedComponent :type Primitive%20Component%20Object%20Reference) (OtherActor :type Actor%20Object%20Reference) (OtherComp :type Primitive%20Component%20Object%20Reference) (OtherBodyIndex :type Integer) (bFromSweep :type Boolean) (SweepResult :type Hit%20Result%20Structure%20%28by%20ref%29))
  (Utilities|Casting|CastTo2DSideScrollerCharacter OtherActor)
  (Variables|Default|SetNomove false)
  (Variables|Default|SetSeePlayer true)
  (CallFunction|TireFusil))

(event OnComponentBeginOverlap(ColliderAR)
  (params (OverlappedComponent :type Primitive%20Component%20Object%20Reference) (OtherActor :type Actor%20Object%20Reference) (OtherComp :type Primitive%20Component%20Object%20Reference) (OtherBodyIndex :type Integer) (bFromSweep :type Boolean) (SweepResult :type Hit%20Result%20Structure%20%28by%20ref%29))
  (Utilities|Casting|CastTo2DSideScrollerCharacter OtherActor)
  (Variables|Default|SetWaithPlayer false)
  (Variables|Default|SetSeePlayer false)
  (Variables|Default|SetNomove false)
  (Variables|Default|SetIsMovingRight (not (Variables|Default|GetIsMovingRight))))

(event Custom|ImpulseHIT
  (bind _retourner_ (Variables|Default|GetRetourner?))
  (if (Variables|Default|GetIsMovingRight)
    (Variables|Default|SetImpulse "-300.000000, 0,300.000000")
    (if (not _retourner_)
      (Variables|Default|SetImpulse "300.000000, 0,300.000000"))
    (else
      (Variables|Default|SetImpulse "300.000000, 0,300.000000")
      (if (not _retourner_)
        (Variables|Default|SetImpulse "-300.000000, 0,300.000000")))))

(event Custom|TireFusil
  (Utilities|FlowControl|DoOnce false
    (:Completed
      (Variables|/Script/Engine.CharacterMovementComponent|SetMaxWalkSpeed (Variables|Character|GetCharacterMovement) 0.0)
      (Variables|Default|SetAnimState "NewEnumerator3")
      (CallFunction|AnimationUpdate)
      (Utilities|FlowControl|Delay 0.3)
      (Game|SpawnActorfromClass "/Game/Enemies/Bullet/Bullet_Blueprint.Bullet_Blueprint_C" (Transformation|GetWorldTransform (Variables|Default|GetScene)) "Undefined" 0 0)
      (Variables|Default|SetAnimState "NewEnumerator0")
      (CallFunction|AnimationUpdate)
      (Utilities|FlowControl|Delay 2.0)
      (CallFunction|ResetBullet))))

(event Custom|AttackUpdate
  (bind _charactermovement (Variables|Character|GetCharacterMovement))
  (Variables|/Script/Engine.CharacterMovementComponent|SetMaxWalkSpeed _charactermovement 0.0)
  (Variables|Default|SetAnimState "NewEnumerator3")
  (Utilities|Casting|CastTo2DSideScrollerCharacter (Game|GetPlayerCharacter 0))
  (if (< (Variables|Default|GetDistance) 8e+02)
    (Utilities|FlowControl|Delay 0.2)
    (if (not (Variables|Default|GetIsDead))
      (Utilities|FlowControl|Delay 0.0)
      (CallFunction|AttackUpdate))
    (else
      (Utilities|FlowControl|Delay 0.0)
      (Variables|/Script/Engine.CharacterMovementComponent|SetMaxWalkSpeed _charactermovement (Variables|Default|GetVitesse))
      (Variables|Default|SetAnimState "NewEnumerator2"))))

(event Custom|Direction
  (if (not (Variables|Default|GetNomove))
    (Transformation|SetRelativeRotation (Variables|Default|GetSprite) (Math|Rotator|MakeRotator 0.0 0.0 (Math|Float|SelectFloat 0.0 1.8e+02 (Variables|Default|GetIsMovingRight))) false false)
    (Pawn|Input|AddMovementInput (Math|Vector|SelectVector (Variables|Default|GetVectorA) (Variables|Default|GetVector%20B) (Variables|Default|GetIsMovingRight)) 1.0 false)))

(event Custom|AnimationUpdate
  (switch Utilities|FlowControl|Switch|SwitchonBetteraveAnim (Variables|Default|GetAnimState)
    (:NewEnumerator0
      (if (Variables|Default|GetIsDead) :!label _label
        (Variables|Default|SetAnimState "NewEnumerator1")
        (else
          (Sprite|SetFlipbook (Variables|Default|GetSprite) (select (> (Math|Vector|VectorLength (Transformation|GetVelocity)) 0.0) "/Game/Enemies/Fleur/FleurWalk.FleurWalk" "/Game/Enemies/Fleur/FleurIdle.FleurIdle")))))
    (:NewEnumerator2
      (goto _label))
    (:NewEnumerator1
      (Sprite|SetFlipbook (Variables|Default|GetSprite) "/Game/Enemies/Fleur/FleurDeathJump.FleurDeathJump"))
    (:NewEnumerator3
      (Sprite|SetFlipbook (Variables|Default|GetSprite) "/Game/Enemies/Fleur/FleurFight.FleurFight"))))

(event Custom|AttackPlayer
  (if (Variables|Default|GetIsDead)
    _))

(event Custom|ResetBullet
  (Utilities|FlowControl|DoOnce false) ; enters at Reset
)

(event Custom|DeadCAC
  (Variables|Default|SetIsDead true)
  (Sprite|SetFlipbook (Variables|Default|GetSprite) "/Game/Enemies/Fleur/FleurSuicide.FleurSuicide")
  (Utilities|FlowControl|Delay 1.3)
  (Actor|DestroyActor))

(event Custom|EventDistance
  (bind _as2dside_scroller_character (Utilities|Casting|CastTo2DSideScrollerCharacter (Game|GetPlayerCharacter 0)))
  (Variables|Default|SetDistance (Math|Vector|VectorLength (- (Transformation|GetActorLocation _as2dside_scroller_character) (Transformation|GetActorLocation)))))

(event Custom|Retourner
  (bind _output_get (Variables|Default|SetVectorA "-1.000000,0.000000, 0"))
  (Variables|Default|SetVectorA _output_get)
  (bind _output_get_2 (Variables|Default|SetVector%20B "1.000000, 0, 0"))
  (Variables|Default|SetVector%20B _output_get_2))

(event Collision|EventActorBeginOverlap
  (params (OtherActor :type Actor%20Object%20Reference)))

(event EventBeginPlay
  (Utilities|FlowControl|Sequence
    (:then_0
      (if (Variables|Default|GetRetourner?)
        (CallFunction|Retourner)))
    (:then_1
      (Variables|/Script/Engine.CharacterMovementComponent|SetMaxWalkSpeed (Variables|Character|GetCharacterMovement) (Variables|Default|GetVitesse)))))

(event EventTick
  (params (DeltaSeconds :type Float%20%28single-precision%29))
  (if (not (Variables|Default|GetIsDead))
    (Utilities|FlowControl|Sequence
      (:then_0
        (CallFunction|AnimationUpdate)
        (if (not (Variables|Default|GetWaithPlayer))
          (CallFunction|Direction)))
      (:then_1
        (CallFunction|EventDistance)
        (CallFunction|ImpulseHIT))
      (:then_2
        (if (Variables|Default|GetSeePlayer)
          (CallFunction|TireFusil))))))

(fn ConstructionScript)

(fn NewFunction0
  (params (IsDeath :type Boolean))
  (return "/Game/Enemies/Betterave/DeathBeterrave.DeathBeterrave"))