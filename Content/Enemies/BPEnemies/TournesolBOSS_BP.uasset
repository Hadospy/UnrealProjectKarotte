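; Paper2D sunflower boss (TournesolBOSS) for a side-scroller that faces the player and fires seed projectiles.
; Tick updates the flipbook from AnimStates and schedules random attacks after random delays.
; The seed attack recursively spawns up to ten PepinProjectil_BP at random spawn points, gated by the shoot animation flag.
; Three overlap zones set the idle direction between attacks; other attacks are print-only stubs, two of them unreachable.
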(event OnComponentBeginOverlap(DetectionDroite)
  (params (OverlappedComponent :type Primitive%20Component%20Object%20Reference) (OtherActor :type Actor%20Object%20Reference) (OtherComp :type Primitive%20Component%20Object%20Reference) (OtherBodyIndex :type Integer) (bFromSweep :type Boolean) (SweepResult :type Hit%20Result%20Structure%20%28by%20ref%29))
  (if (not (Variables|Default|GetAttaque?))
    (Utilities|Casting|CastTo2DSideScrollerCharacter OtherActor)
    (Variables|Default|SetJoueur%20Droite true)
    (Variables|Default|SetJoueur%20Devant false)
    (Variables|Default|SetJoueur%20Gauche false)
    (Variables|Default|SetAnimStates "NewEnumerator1")))

(event OnComponentBeginOverlap(Detectiondevant)
  (params (OverlappedComponent :type Primitive%20Component%20Object%20Reference) (OtherActor :type Actor%20Object%20Reference) (OtherComp :type Primitive%20Component%20Object%20Reference) (OtherBodyIndex :type Integer) (bFromSweep :type Boolean) (SweepResult :type Hit%20Result%20Structure%20%28by%20ref%29))
  (if (not (Variables|Default|GetAttaque?))
    (Utilities|Casting|CastTo2DSideScrollerCharacter OtherActor)
    (Variables|Default|SetJoueur%20Droite false)
    (Variables|Default|SetJoueur%20Devant true)
    (Variables|Default|SetJoueur%20Gauche false)
    (Variables|Default|SetAnimStates "NewEnumerator0")))

(event OnComponentBeginOverlap(DetectionGauche)
  (params (OverlappedComponent :type Primitive%20Component%20Object%20Reference) (OtherActor :type Actor%20Object%20Reference) (OtherComp :type Primitive%20Component%20Object%20Reference) (OtherBodyIndex :type Integer) (bFromSweep :type Boolean) (SweepResult :type Hit%20Result%20Structure%20%28by%20ref%29))
  (if (not (Variables|Default|GetAttaque?))
    (Utilities|Casting|CastTo2DSideScrollerCharacter OtherActor)
    (Variables|Default|SetJoueur%20Droite false)
    (Variables|Default|SetJoueur%20Devant false)
    (Variables|Default|SetJoueur%20Gauche true)
    (Variables|Default|SetAnimStates "NewEnumerator2")))

(event Custom|UpdateAnim
  (bind _sprite (Variables|Default|GetSprite))
  ;[1 1 1] Update Anim
  (switch Utilities|FlowControl|Switch|SwitchonBossTournesolStep (Variables|Default|GetAnimStates)
    (:NewEnumerator0
      (Sprite|SetFlipbook _sprite "/Game/Boss/BossKarrotteIdle.BossKarrotteIdle"))
    (:NewEnumerator1
      (Sprite|SetFlipbook _sprite "/Game/Boss/BossKarrotteIdleR.BossKarrotteIdleR"))
    (:NewEnumerator2
      (Sprite|SetFlipbook _sprite "/Game/Boss/BossKarrotteIdleG.BossKarrotteIdleG"))
    (:NewEnumerator3
      (if (Variables|Default|GetAttaquePepin)
        (Utilities|FlowControl|DoOnce false :!label _label
          (:Completed
            (Sprite|SetFlipbook _sprite "/Game/Boss/BossKarrotteIdleTir.BossKarrotteIdleTir")
            (Utilities|FlowControl|Delay 1.8)
            (Variables|Default|SetAnimTir true)
            (Variables|Default|SetAnimStates "NewEnumerator0")))
        (else
          (goto _label Reset))))))

(event Custom|RandomAttack
  (Utilities|FlowControl|Delay 1.0)
  (Utilities|Time|SetTimerbyEvent (delegate Custom|Attack%20Finish) 0.5 true)
  (switch int (Math|Random|RandomIntegerinRange 0 1)
    (:0
      (CallFunction|AttaquePEPIN)
      (Development|PrintString "Attack 1")
      (Utilities|FlowControl|Delay 3.0)
      (CallFunction|AttackFinish)
      (Variables|Default|SetAttaque? false))
    (:1
      (Development|PrintString "Attack 2")
      (Utilities|FlowControl|Delay 3.0)
      (CallFunction|AttackFinish)
      (Variables|Default|SetAttaque? false))
    (:2
      (Development|PrintString "Attack3")
      (Utilities|FlowControl|Delay 3.0)
      (CallFunction|AttackFinish)
      (Variables|Default|SetAttaque? false))
    (:3
      (Development|PrintString "Attack 4")
      (Utilities|FlowControl|Delay 3.0)
      (CallFunction|AttackFinish)
      ;[1 1 1] AttquePepin
      (Variables|Default|SetAttaque? false))))

(event Custom|Attack%20Finish)

(event Custom|ResetTir
  ;[1 1 1] AttquePepin
  (if (and (< (Variables|Default|GetNombrePepinTir) 10) (Variables|Default|GetAttaquePepin))
    (Utilities|FlowControl|Delay 0.3)
    (Game|SpawnActorfromClass "/Game/Boss/PepinProjectil_BP.PepinProjectil_BP_C" (Transformation|GetWorldTransform (Utilities|Array|Get(acopy) (Utilities|Array|MakeArray (Variables|Default|GetSpawnPépin4) (Variables|Default|GetSpawnPépin5) (Variables|Default|GetSpawnPépin6) (Variables|Default|GetSpawnPépin7) (Variables|Default|GetSpawnPépin8) (Variables|Default|GetSpawnPépin9) (Variables|Default|GetSpawnPépin10) (Variables|Default|GetSpawnPépin2) (Variables|Default|GetSpawnPépin3) (Variables|Default|GetSpawnPépin11) 0 0 0) (Math|Random|RandomIntegerinRange 0 9))) "Undefined" 0 0)
    (bind _output_get (Variables|Default|SetNombrePepinTir (Variables|Default|GetNombrePepinTir)))
    (bind _result (Math|Integer|IncrementInt _output_get)
      (:%20%20
        (Variables|Default|SetNombrePepinTir _result)
        (CallFunction|ResetTir)))
    (else
      (bind _output_get_2 (Variables|Default|SetNombrePepinTir 0))
      (Variables|Default|SetNombrePepinTir _output_get_2)
      (Variables|Default|SetAttaquePepin false))))

(event Custom|Attaque%20PEPIN
  ;[1 1 1] AttquePepin
  (Variables|Default|SetAttaquePepin true)
  (Variables|Default|SetAnimStates "NewEnumerator3")
  (if (Variables|Default|GetAnimTir)
    (Variables|Default|SetAnimTir false)
    (if (and (< (Variables|Default|GetNombrePepinTir) 10) (Variables|Default|GetAttaquePepin))
      (Utilities|FlowControl|Delay 0.3)
      (Game|SpawnActorfromClass "/Game/Boss/PepinProjectil_BP.PepinProjectil_BP_C" (Transformation|GetWorldTransform (Utilities|Array|Get(acopy) (Utilities|Array|MakeArray (Variables|Default|GetSpawnPépin4) (Variables|Default|GetSpawnPépin5) (Variables|Default|GetSpawnPépin6) (Variables|Default|GetSpawnPépin7) (Variables|Default|GetSpawnPépin8) (Variables|Default|GetSpawnPépin9) (Variables|Default|GetSpawnPépin10) (Variables|Default|GetSpawnPépin2) (Variables|Default|GetSpawnPépin3) (Variables|Default|GetSpawnPépin11) 0 0 0) (Math|Random|RandomIntegerinRange 0 9))) "Undefined" 0 0)
      (bind _output_get (Variables|Default|SetNombrePepinTir (Variables|Default|GetNombrePepinTir)))
      (bind _result (Math|Integer|IncrementInt _output_get)
        (:%20%20
          (Variables|Default|SetNombrePepinTir _result)
          (CallFunction|ResetTir)))
      (else
        (bind _output_get_2 (Variables|Default|SetNombrePepinTir 0))
        (Variables|Default|SetNombrePepinTir _output_get_2)
        (Variables|Default|SetAttaquePepin false)))))

(event EventBeginPlay)

(event Collision|EventActorBeginOverlap
  (params (OtherActor :type Actor%20Object%20Reference)))

(event EventTick
  (params (DeltaSeconds :type Float%20%28single-precision%29))
  (Utilities|FlowControl|Sequence
    (:then_0
      (CallFunction|UpdateAnim))
    (:then_1
      (if (not (Variables|Default|GetAttaque?))
        (Variables|Default|SetAttaque? true)
        (Utilities|FlowControl|Delay (Math|Random|RandomFloatinRange 1.0 3.0))
        (CallFunction|RandomAttack)))))

(fn ConstructionScript)