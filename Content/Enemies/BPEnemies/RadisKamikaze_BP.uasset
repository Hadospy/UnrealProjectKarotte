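; Kamikaze radish enemy for a 2D side-scroller that walks along and explodes near the player, launching and damaging them.
; Tick drives movement, flipbook state, player distance and line traces that reverse it at certain actors or start the attack.
; Vision and rear overlaps track the player, while collision hits trigger gated turnarounds.
; The attack speeds up, then explodes after a delay; DeadCAC detonates immediately without a distance check.
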(event OnComponentBeginOverlap(ColliderAr)
  (params (OverlappedComponent :type Primitive%20Component%20Object%20Reference) (OtherActor :type Actor%20Object%20Reference) (OtherComp :type Primitive%20Component%20Object%20Reference) (OtherBodyIndex :type Integer) (bFromSweep :type Boolean) (SweepResult :type Hit%20Result%20Structure%20%28by%20ref%29))
  (bind _charactermovement (Variables|Character|GetCharacterMovement))
  ;[1 1 1] Detection Collider Arrière
  (Utilities|Casting|CastTo2DSideScrollerCharacter OtherActor)
  (Variables|Default|SetSeePlayer true)
  (Variables|Default|SetNomove false)
  (Utilities|FlowControl|DoOnce false
    (:Completed
      (Variables|/Script/Engine.CharacterMovementComponent|SetMaxWalkSpeed _charactermovement 0.0)
      (Variables|Default|SetIsMovingRight (not (Variables|Default|GetIsMovingRight)))
      (Utilities|FlowControl|Delay 0.2)
      (Variables|/Script/Engine.CharacterMovementComponent|SetMaxWalkSpeed _charactermovement (Variables|Default|GetVitesse)))))

(event OnComponentHit(CapsuleComponent)
  (params (HitComponent :type Primitive%20Component%20Object%20Reference) (OtherActor :type Actor%20Object%20Reference) (OtherComp :type Primitive%20Component%20Object%20Reference) (NormalImpulse :type Vector :default "0, 0, 0") (Hit :type Hit%20Result%20Structure%20%28by%20ref%29))
  (bind _charactermovement (Variables|Character|GetCharacterMovement))
  ;[1 1 1] Hit Obstacle Demi tour
  (if (not (Variables|Default|GetAttack))
    (if (not (Variables|Default|GetSeePlayer))
      (Utilities|FlowControl|DoOnce false
        (:Completed
          (Variables|/Script/Engine.CharacterMovementComponent|SetMaxWalkSpeed _charactermovement 0.0)
          (Variables|Default|SetIsMovingRight (not (Variables|Default|GetIsMovingRight)))
          (Utilities|FlowControl|Delay 0.2)
          (Variables|/Script/Engine.CharacterMovementComponent|SetMaxWalkSpeed _charactermovement (Variables|Default|GetVitesse))
          (Utilities|FlowControl|Delay 1.0)
          (CallFunction|ResetDemitour))))))

(event OnComponentHit(ColliderJump)
  (params (HitComponent :type Primitive%20Component%20Object%20Reference) (OtherActor :type Actor%20Object%20Reference) (OtherComp :type Primitive%20Component%20Object%20Reference) (NormalImpulse :type Vector :default "0, 0, 0") (Hit :type Hit%20Result%20Structure%20%28by%20ref%29))
  (bind _charactermovement (Variables|Character|GetCharacterMovement))
  ;[1 1 1] Hit Obstacle Demi tour
  (if (not (Variables|Default|GetAttack))
    (if (not (Variables|Default|GetSeePlayer))
      (Utilities|FlowControl|DoOnce false
        (:Completed
          (Variables|/Script/Engine.CharacterMovementComponent|SetMaxWalkSpeed _charactermovement 0.0)
          (Variables|Default|SetIsMovingRight (not (Variables|Default|GetIsMovingRight)))
          (Utilities|FlowControl|Delay 0.2)
          (Variables|/Script/Engine.CharacterMovementComponent|SetMaxWalkSpeed _charactermovement (Variables|Default|GetVitesse))
          (Utilities|FlowControl|Delay 1.0)
          (CallFunction|ResetDemitour))))))

(event OnComponentEndOverlap(ColliderAr)
  (params (OverlappedComponent :type Primitive%20Component%20Object%20Reference) (OtherActor :type Actor%20Object%20Reference) (OtherComp :type Primitive%20Component%20Object%20Reference) (OtherBodyIndex :type Integer))
  ;[1 1 1] Sorti Champ vision BoxArriere
  (Utilities|Casting|CastTo2DSideScrollerCharacter OtherActor)
  (Variables|Default|SetSeePlayer false)
  (Utilities|FlowControl|Delay 1.0)
  (Utilities|FlowControl|Sequence
    (:then_0
      (CallFunction|Resetdetect))
    (:then_1
      (CallFunction|ResetDemitour))))

(event OnComponentEndOverlap(ChampDeVision)
  (params (OverlappedComponent :type Primitive%20Component%20Object%20Reference) (OtherActor :type Actor%20Object%20Reference) (OtherComp :type Primitive%20Component%20Object%20Reference) (OtherBodyIndex :type Integer))
  ;[1 1 1] Sorti Champ vison Enemi
  (Utilities|Casting|CastTo2DSideScrollerCharacter OtherActor)
  (Variables|Default|SetSeePlayer false)
  (Utilities|FlowControl|Delay 1.0)
  (Utilities|FlowControl|Sequence
    (:then_0
      (CallFunction|Resetdetect))
    (:then_1
      (CallFunction|ResetDemitour))))

(event OnComponentBeginOverlap(ChampDeVision)
  (params (OverlappedComponent :type Primitive%20Component%20Object%20Reference) (OtherActor :type Actor%20Object%20Reference) (OtherComp :type Primitive%20Component%20Object%20Reference) (OtherBodyIndex :type Integer) (bFromSweep :type Boolean) (SweepResult :type Hit%20Result%20Structure%20%28by%20ref%29))
  ;[1 1 1] Champs Vision Enemi
  (Utilities|Casting|CastTo2DSideScrollerCharacter OtherActor)
  (Variables|Default|SetSeePlayer true)
  (Variables|Default|SetNomove false))

(event Custom|ImpulseHIT
  (bind _retourner_ (Variables|Default|GetRetourner?))
  ;[1 1 1] Impulse Joueur
  (if (Variables|Default|GetIsMovingRight)
    (Variables|Default|SetImpulse "-300.000000, 0,300.000000")
    (if (not _retourner_)
      (Variables|Default|SetImpulse "300.000000, 0,300.000000"))
    (else
      (Variables|Default|SetImpulse "300.000000, 0,300.000000")
      (if (not _retourner_)
        (Variables|Default|SetImpulse "-300.000000, 0,300.000000")))))

(event Custom|DetecteEnemi
  (bind _charactermovement (Variables|Character|GetCharacterMovement))
  (bind _sprite (Variables|Default|GetSprite))
  (bind _returnvalue (Transformation|GetWorldLocation _sprite))
  ;[1 1 1] DetecteEnemi Demi Tour RAYCAST
  (if (not (Variables|Default|GetIsDead))
    (bind (_outhit _returnvalue_2) (Collision|LineTraceByChannel _returnvalue (+ _returnvalue (* (Math|Vector|GetForwardVector _sprite) 1.2e+02)) "TraceTypeQuery1" false 0 "None"))
    (if _returnvalue_2
      (Utilities|FlowControl|Sequence
        (:then_0
          (Utilities|Casting|CastToBetteRave_BP (.HitActor (Collision|BreakHitResult _outhit))))
        (:then_1
          (Utilities|Casting|CastToCacarnivor_Blueprint1 (.HitActor (Collision|BreakHitResult _outhit))))
        (:then_2
          (Utilities|Casting|CastToRadisKamikaze_BP (.HitActor (Collision|BreakHitResult _outhit))))
        (:then_3
          (Utilities|Casting|CastToChampignon_Blueprint (.HitActor (Collision|BreakHitResult _outhit))))
        (:then_4
          (Utilities|Casting|CastToTruelleCheckpoint_BP (.HitActor (Collision|BreakHitResult _outhit)))))
      (Variables|/Script/Engine.CharacterMovementComponent|SetMaxWalkSpeed _charactermovement 0.0)
      (if (not (Variables|Default|GetSeePlayer))
        (Utilities|FlowControl|Delay 0.3)
        (Variables|Default|SetIsMovingRight (not (Variables|Default|GetIsMovingRight)))
        (Variables|/Script/Engine.CharacterMovementComponent|SetMaxWalkSpeed _charactermovement (Variables|Default|GetVitesse))))))

(event Custom|Kamikaze
  ;[1 1 1] Kamikaze
  (Audio|PlaySound2D "/Game/Son/Explosion.Explosion")
  (bind _as2dside_scroller_character (Utilities|Casting|CastTo2DSideScrollerCharacter (Game|GetPlayerCharacter 0)))
  (Variables|Default|SetIsDead true)
  (Variables|Default|SetAnimState "NewEnumerator1")
  (CallFunction|AnimationUpdate)
  (Character|LaunchCharacter _as2dside_scroller_character (Variables|Default|GetImpulse) true true)
  (Default|HealthDown _as2dside_scroller_character)
  (Utilities|FlowControl|Delay 0.5)
  (Actor|DestroyActor))

(event Custom|AttackUpdate
  ;[1 1 1] Check Attaque Joueur
  (Utilities|FlowControl|DoOnce false
    (:Completed
      (Variables|Default|SetAnimState "NewEnumerator3")
      (Variables|/Script/Engine.CharacterMovementComponent|SetMaxWalkSpeed (Variables|Character|GetCharacterMovement) 4e+02)
      (bind _as2dside_scroller_character (Utilities|Casting|CastTo2DSideScrollerCharacter (Game|GetPlayerCharacter 0)))
      (Utilities|FlowControl|Delay 0.6)
      (Audio|PlaySound2D "/Game/Son/Explosion.Explosion")
      (if (< (Variables|Default|GetDistance) 3e+02)
        (Utilities|FlowControl|Delay 0.1)
        (if (not (Variables|Default|GetIsDead))
          (Character|LaunchCharacter _as2dside_scroller_character (Variables|Default|GetImpulse) true true)
          (Default|HealthDown _as2dside_scroller_character)
          (Utilities|FlowControl|Delay 0.9)
          (Actor|DestroyActor))
        (else
          (Utilities|FlowControl|Delay 1.0)
          (Actor|DestroyActor))))))

(event Custom|AttackPlayer
  (bind _sprite (Variables|Default|GetSprite))
  (bind _returnvalue (Transformation|GetWorldLocation _sprite))
  ;[1 1 1] Raycast AttackPlayer
  (if (not (Variables|Default|GetIsDead))
    (bind (_outhit _returnvalue_2) (Collision|LineTraceByChannel _returnvalue (+ _returnvalue (* (Math|Vector|GetForwardVector _sprite) 1.3e+02)) "TraceTypeQuery1" false 0 "None"))
    (if _returnvalue_2
      (Utilities|FlowControl|Sequence
        (:then_0
          (Utilities|Casting|CastTo2DSideScrollerCharacter (.HitActor (Collision|BreakHitResult _outhit)))
          (Variables|Default|SetAttack true)
          (Utilities|FlowControl|Delay 0.0)
          (Utilities|FlowControl|DoOnce false
            (:Completed
              (if (not (Variables|Default|GetIsDead))
                (CallFunction|AttackUpdate)))))))))

(event Custom|Direction
  ;[1 1 1] Direction
  (if (not (Variables|Default|GetNomove))
    (if (not (Variables|Default|GetNoMove&NoTurn))
      (Transformation|SetRelativeRotation (Variables|Default|GetSprite) (Math|Rotator|MakeRotator 0.0 0.0 (Math|Float|SelectFloat 0.0 1.8e+02 (Variables|Default|GetIsMovingRight))) false false)
      (Pawn|Input|AddMovementInput (Math|Vector|SelectVector (Variables|Default|GetVectorA) (Variables|Default|GetVector%20B) (Variables|Default|GetIsMovingRight)) 1.0 false))))

(event Custom|AnimationUpdate
  (bind _sprite (Variables|Default|GetSprite))
  ;[1 1 1] Animation Update
  (switch Utilities|FlowControl|Switch|SwitchonBetteraveAnim (Variables|Default|GetAnimState)
    (:NewEnumerator0
      (if (Variables|Default|GetIsDead) :!label _label
        (Variables|Default|SetAnimState "NewEnumerator1")
        (else
          (Sprite|SetFlipbook _sprite (select (> (Math|Vector|VectorLength (Transformation|GetVelocity)) 0.0) "/Game/Enemies/Radis/RadisWalk.RadisWalk" "/Game/Enemies/Radis/RadisIdle.RadisIdle")))))
    (:NewEnumerator2
      (goto _label))
    (:NewEnumerator1
      (Sprite|SetFlipbook _sprite "/Game/Enemies/Radis/RadisKamiakaze2.RadisKamiakaze2"))
    (:NewEnumerator3
      (Sprite|SetFlipbook _sprite "/Game/Enemies/Radis/RadisKamkikaze.RadisKamkikaze"))))

(event Custom|Resetdetect
  (bind _charactermovement (Variables|Character|GetCharacterMovement))
  ;[1 1 1] Detection Collider Arrière
  (Utilities|FlowControl|DoOnce false) ; enters at Reset
)

(event Custom|Reset
  ;[1 1 1] Raycast AttackPlayer
  (Utilities|FlowControl|DoOnce false) ; enters at Reset
)

(event Custom|AttackUp
  (bind _sprite (Variables|Default|GetSprite))
  (bind _returnvalue (Transformation|GetWorldLocation _sprite))
  ;[1 1 1] RaycastUpVector
  (if (not (Variables|Default|GetIsDead))
    (Utilities|FlowControl|Sequence
      (:then_0
        (bind (_outhit _returnvalue_2) (Collision|LineTraceByChannel _returnvalue (+ _returnvalue (* (Math|Vector|GetUpVector _sprite) 2e+02)) "TraceTypeQuery1" false 0 "None"))
        (if _returnvalue_2
          (Utilities|FlowControl|Sequence
            (:then_0
              (Utilities|Casting|CastTo2DSideScrollerCharacter (.HitActor (Collision|BreakHitResult _outhit)))
              (Utilities|FlowControl|DoOnce false
                (:Completed
                  (CallFunction|AttackUpdate))))
            (:then_1
              (Utilities|Casting|CastToBetteRave_BP (.HitActor (Collision|BreakHitResult _outhit)))
              (Variables|Default|SetIsMovingRight (not (Variables|Default|GetIsMovingRight))))))))))

(event Custom|DeadCAC
  ;[1 1 1] CAC mort enemi
  (Variables|Default|SetIsDead true)
  (CallFunction|Kamikaze))

(event Custom|EventDistance
  ;[1 1 1] Recupere Distance Joueur
  (bind _as2dside_scroller_character (Utilities|Casting|CastTo2DSideScrollerCharacter (Game|GetPlayerCharacter 0)))
  (Variables|Default|SetDistance (Math|Vector|VectorLength (- (Transformation|GetActorLocation _as2dside_scroller_character) (Transformation|GetActorLocation)))))

(event Custom|Retourner
  ;[1 1 1] Retourner Sprite
  (bind _output_get (Variables|Default|SetVectorA "-1.000000,0.000000, 0"))
  (Variables|Default|SetVectorA _output_get)
  (bind _output_get_2 (Variables|Default|SetVector%20B "1.000000,0.000000, 0"))
  (Variables|Default|SetVector%20B _output_get_2))

(event Custom|ResetDemitour
  (bind _charactermovement (Variables|Character|GetCharacterMovement))
  ;[1 1 1] Hit Obstacle Demi tour
  (Utilities|FlowControl|DoOnce false) ; enters at Reset
)

(event EventBeginPlay
  ;[1 1 1] Begin Play
  (Utilities|FlowControl|Sequence
    (:then_0
      (if (Variables|Default|GetRetourner?)
        (CallFunction|Retourner)))
    (:then_1
      (Variables|/Script/Engine.CharacterMovementComponent|SetMaxWalkSpeed (Variables|Character|GetCharacterMovement) (Variables|Default|GetVitesse)))))

(event EventTick
  (params (DeltaSeconds :type Float%20%28single-precision%29))
  ;[1 1 1] Event Tick
  (if (not (Variables|Default|GetIsDead))
    (Utilities|FlowControl|Sequence
      (:then_0
        (CallFunction|AttackPlayer)
        (CallFunction|Direction)
        (CallFunction|AnimationUpdate)
        (CallFunction|AttackUp))
      (:then_1
        (CallFunction|EventDistance)
        (CallFunction|ImpulseHIT)
        (CallFunction|DetecteEnemi)))))

(fn ConstructionScript
  (Transformation|SetRelativeScale3D (Variables|Default|GetChampDeVision) (Math|Vector|MakeVector 1.25 2.0 (Variables|Default|GetSizeChampDeVision))))

(fn NewFunction0
  (params (IsDeath :type Boolean))
  (return "/Game/Enemies/Betterave/DeathBeterrave.DeathBeterrave"))