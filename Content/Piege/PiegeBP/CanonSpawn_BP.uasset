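; CanonSpawn_BP is a spawner cannon trap that repeatedly spawns one selected enemy type while Activate is set.
; Tick calls SpawnEnemies, which enters a DoOnce gate and spawns Radis Kamikaze, Cacarnivor, Patates or Bettraves at the Spawn component's transform, chosen by the Enemies enum.
; After a TempsSpawn delay, ResetSpawn reopens the gate, so the delay paces the spawn loop.
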(event Custom|SpawnEnemies
  (bind _spawn (Variables|Default|GetSpawn))
  (bind _returnvalue (Transformation|GetWorldTransform _spawn))
  (Utilities|FlowControl|DoOnce false
    (:Completed
      (switch Utilities|FlowControl|Switch|SwitchonSpawnChoices (Variables|Default|GetEnemies)
        (:NewEnumerator0
          (Game|SpawnActorfromClass "/Game/Enemies/BPEnemies/RadisKamikaze_BP.RadisKamikaze_BP_C" _returnvalue "AdjustIfPossibleButAlwaysSpawn" 0 0))
        (:NewEnumerator1
          (Game|SpawnActorfromClass "/Game/Enemies/BPEnemies/Cacarnivor_Blueprint1.Cacarnivor_Blueprint1_C" _returnvalue "AdjustIfPossibleButAlwaysSpawn" 0 0))
        (:NewEnumerator2
          (Game|SpawnActorfromClass "/Game/Enemies/BPEnemies/Patate_BP.Patate_BP_C" _returnvalue "AdjustIfPossibleButAlwaysSpawn" 0 0))
        (:NewEnumerator3
          (Game|SpawnActorfromClass "/Game/Enemies/BPEnemies/BetteRave_BP.BetteRave_BP_C" _returnvalue "AdjustIfPossibleButAlwaysSpawn" 0 0)))
      (Utilities|FlowControl|Delay (Variables|Default|GetTemps%20spawn))
      (CallFunction|ResetSpawn))))

(event Custom|ResetSpawn
  (bind _spawn (Variables|Default|GetSpawn))
  (bind _returnvalue (Transformation|GetWorldTransform _spawn))
  (Utilities|FlowControl|DoOnce false) ; enters at Reset
)

(event EventTick
  (params (DeltaSeconds :type Float%20%28single-precision%29))
  (if (Variables|Default|GetActivate?)
    (CallFunction|SpawnEnemies)))

(fn ConstructionScript)