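; Cannon trap that repeatedly spawns kamikaze radish actors (RadisKamikaze_BP) at its Spawn component's transform.
; Tick calls Spawnradie every frame, but a DoOnce gate lets only one spawn through per cycle.
; Each spawn is stored in Radis, then a TempsSpawn delay calls Resetspawn to reopen the gate.
; Spawning is skipped when the spawn point is colliding.
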(event Custom|Spawn%20radie
  (Utilities|FlowControl|DoOnce false
    (:Completed
      (bind _returnvalue (Game|SpawnActorfromClass "/Game/Enemies/BPEnemies/RadisKamikaze_BP.RadisKamikaze_BP_C" (Transformation|GetWorldTransform (Variables|Default|GetSpawn)) "DontSpawnIfColliding" 0 0))
      (Variables|Default|SetRadis _returnvalue)
      (Utilities|FlowControl|Delay (Variables|Default|GetTemps%20spawn))
      (CallFunction|ResetSpawn))))

(event Custom|Reset%20spawn
  (Utilities|FlowControl|DoOnce false) ; enters at Reset
)

(event EventTick
  (params (DeltaSeconds :type Float%20%28single-precision%29))
  (CallFunction|SpawnRadie))

(fn ConstructionScript)